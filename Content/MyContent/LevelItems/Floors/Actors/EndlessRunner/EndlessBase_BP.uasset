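; EndlessBase_BP is a floor segment for an endless runner side-scroller that chains the next segment at runtime.
; One second after the character overlaps Collision, it spawns a random segment at the Arrow's transform.
; The switch lists itself and three EndlessFloor variants, but the random range only reaches EndlessBase_BP and EndlessFloor1_BP.
; Ending overlap with KillBox sets the character's Dead flag.
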(event `self.Collision.OnComponentBeginOverlap`
  (params (OverlappedComponent :type "PrimitiveComponent Object Reference") (OtherActor :type "Actor Object Reference") (OtherComp :type "PrimitiveComponent Object Reference") (OtherBodyIndex :type Integer) (bFromSweep :type Boolean) (SweepResult :type "HitResult Structure (by ref)"))
  (cast `/Game/MyContent/Characters/NinjaCharacter/EndlessRunnerSideScrollerCharacter` OtherActor)
  (`KismetSystemLibrary.Delay` 1.0)
  (switch `int` (`KismetMathLibrary.RandomIntegerInRange` 0 1)
    (:`0`
      (`|SpawnActorFromClass` "EndlessBase_BP_C" (`SceneComponent.K2_GetComponentToWorld` (`self.Arrow`)) "AlwaysSpawn" "OverrideRootScale" null null))
    (:`1`
      (`|SpawnActorFromClass` "/Game/MyContent/LevelItems/Floors/Actors/EndlessRunner/EndlessFloor1_BP.EndlessFloor1_BP_C" (`SceneComponent.K2_GetComponentToWorld` (`self.Arrow`)) "AlwaysSpawn" "OverrideRootScale" null null))
    (:`2`
      (`|SpawnActorFromClass` "/Game/MyContent/LevelItems/Floors/Actors/EndlessRunner/EndlessFloor2_BP.EndlessFloor2_BP_C" (`SceneComponent.K2_GetComponentToWorld` (`self.Arrow`)) "AlwaysSpawn" "OverrideRootScale" null null))
    (:`3`
      (`|SpawnActorFromClass` "/Game/MyContent/LevelItems/Floors/Actors/EndlessRunner/EndlessFloor3_BP.EndlessFloor3_BP_C" (`SceneComponent.K2_GetComponentToWorld` (`self.Arrow`)) "AlwaysSpawn" "OverrideRootScale" null null))))

(event `self.KillBox.OnComponentEndOverlap`
  (params (OverlappedComponent :type "PrimitiveComponent Object Reference") (OtherActor :type "Actor Object Reference") (OtherComp :type "PrimitiveComponent Object Reference") (OtherBodyIndex :type Integer))
  (bind _asendless_runner_side_scroller_character (cast `/Game/MyContent/Characters/NinjaCharacter/EndlessRunnerSideScrollerCharacter` OtherActor))
  (set `/Game/MyContent/Characters/NinjaCharacter/EndlessRunnerSideScrollerCharacter.Dead` true _asendless_runner_side_scroller_character))

(fn `UserConstructionScript`)