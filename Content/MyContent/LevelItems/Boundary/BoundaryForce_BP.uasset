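; Boundary level item that pushes bubbles inside its volume with a configurable force.
; Begin and end overlap events on the Boundary component add and remove cast-matched actors in a Bubbles array.
; Each Tick applies ForceAmount to every tracked bubble's collision as an acceleration change, so the push ignores mass.
; An impulse variant and a debug print remain as unconnected nodes.
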(event `ApplyForceToBubble`
  (params (Bubble :type "Object Object Reference"))
  (`PrimitiveComponent.AddForce` (`/Game/MyContent/LevelItems/Boundary/BoundaryForce_BP.BubbleCollision` Bubble) (`self.ForceAmount`) "None" true))

(event `self.Boundary.OnComponentBeginOverlap`
  (params (OverlappedComponent :type "PrimitiveComponent Object Reference") (OtherActor :type "Actor Object Reference") (OtherComp :type "PrimitiveComponent Object Reference") (OtherBodyIndex :type Integer) (bFromSweep :type Boolean) (SweepResult :type "HitResult Structure (by ref)"))
  (bind _asphysics_bubble_bp (cast `` OtherActor))
  (`KismetArrayLibrary.Array_Add` (`self.Bubbles`) _asphysics_bubble_bp))

(event `self.Boundary.OnComponentEndOverlap`
  (params (OverlappedComponent :type "PrimitiveComponent Object Reference") (OtherActor :type "Actor Object Reference") (OtherComp :type "PrimitiveComponent Object Reference") (OtherBodyIndex :type Integer))
  (bind _asphysics_bubble_bp (cast `` OtherActor))
  (`KismetArrayLibrary.Array_RemoveItem` (`self.Bubbles`) _asphysics_bubble_bp))

(event `self.ReceiveTick`
  (params (DeltaSeconds :type "Float (single-precision)"))
  (for _array_element (`self.Bubbles`)
    (`self.ApplyForceToBubble` _array_element)))

(fn `UserConstructionScript`)