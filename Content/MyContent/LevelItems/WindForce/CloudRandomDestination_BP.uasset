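; A Paper2D cloud character that drifts on the X/Z plane toward random destinations while carrying a radial force, apparently as a wind hazard.
; Looping timers pick new destinations and spawn markers at them, and Tick feeds the offset into movement input.
; BeginPlay applies the force settings, and text components display strength values.
; A death branch exists, but the logic setting its flag is unconnected.
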(event `self.ReceiveBeginPlay`
  ;[1 1 1] BeginPlay - Set Destination Timer
  (`self.SetDestination`)
  (`self.ShowDestinationMarker`)
  (`KismetSystemLibrary.K2_SetTimer` null "SetDestination" 5.0 true)
  (`KismetSystemLibrary.Delay` 0.2)
  (`KismetSystemLibrary.K2_SetTimer` null "ShowDestinationMarker" 3.0 true)
  (`self.DisplayForces`)
  (`self.SetForces`))

(event `UpdateAnimation`
  ;[1 1 1] Handle Animation
  (if (`NavMovementComponent.IsFalling` (`self.CharacterMovement`))
    (`PaperFlipbookComponent.SetFlipbook` (`self.Sprite`) "/Game/MyContent/Textures/Props/Cloud_Flipbook.Cloud_Flipbook")
    (else
      (`PaperFlipbookComponent.SetFlipbook` (`self.Sprite`) (select `bool` (> (`KismetMathLibrary.VSize` (`self.GetVelocity`)) 0.0) :`false` "/Game/MyContent/Textures/Props/Cloud_Flipbook.Cloud_Flipbook" :`true` "/Game/MyContent/Textures/Props/Cloud_Flipbook.Cloud_Flipbook" :!type "PaperFlipbook Object Reference")))))

(event `InputAxis|MoveRight`
  (params (AxisValue :type "Float (single-precision)"))
  ;[1 1 1] Handle movement
  (if (> AxisValue 0.0)
    (set `self.bisMovingRight` true)
    (elif (< AxisValue 0.0)
      (set `self.bisMovingRight` false)))
  (`self.AddMovementInput` (1.0 0.0 0.0) AxisValue))

(event `self.ReceiveTick`
  (params (DeltaSeconds :type "Float (single-precision)"))
  (bind (_destination_x _destination_y _destination_z) (`KismetMathLibrary.BreakVector` (`self.Destination`)))
  (bind _destination_x_2 (`KismetMathLibrary.BreakVector` (`self.Destination`)))
  (bind (_returnvalue_x _returnvalue_y _returnvalue_z) (`KismetMathLibrary.BreakVector` (`SceneComponent.K2_GetComponentLocation` (`self.CapsuleComponent`))))
  (bind _returnvalue_x_2 (`KismetMathLibrary.BreakVector` (`SceneComponent.K2_GetComponentLocation` (`self.CapsuleComponent`))))
  (bind _returnvalue (- _destination_z _returnvalue_z))
  (bind _returnvalue_2 (- _destination_x_2 _returnvalue_x_2))
  ;[1 1 1] Tick - Updates animation
  ;;[1 1 1] Am I dead, play death followed by dead animation
  (if (`self.AmIDead`)
    (`/Engine/EditorBlueprintResources/StandardMacros.DoOnce` false
      (:`Completed`
        (`PaperFlipbookComponent.SetFlipbook` (`self.Sprite`) "/Game/MyContent/Textures/Props/Cloud_Flipbook.Cloud_Flipbook")
        (`self.DisableInput` null)
        (`GameplayStatics.PlaySoundAtLocation` null (`SceneComponent.K2_GetComponentLocation` (`self.CapsuleComponent`)) (struct) 1.0 1.0 0.0 null null null)
        (`KismetSystemLibrary.Delay` 1.3)
        (`self.K2_DestroyActor`)))
    (else
      (`self.DisplayForces`)
      (if (not (`self.DestinationReached`))
        (`|ExecutionSequence`
          (:`then_0`
            ;;[1 1 1] Move X Axis (Left/Righr)
            (if (>= _returnvalue_2 0.0)
              (set `self.bisMovingRight` true)
              (else
                (set `self.bisMovingRight` false)))
            (`self.AddMovementInput` (1.0 0.0 0.0) _returnvalue_2))
          (:`then_1`
            ;;[1 1 1] Move Z Axis (Up/Down)
            (if (>= _returnvalue 0.0)
              (set `self.bIsMovingUp` true)
              (else
                (set `self.bIsMovingUp` false)))
            (`self.AddMovementInput` (0.0 0.0 1.0) _returnvalue)))
        (else
          ;;[1 1 1] Update movement animation
          (`self.UpdateAnimation`)
          (`/Engine/EditorBlueprintResources/StandardMacros.CompareFloat` (.x (`MovementComponent.Velocity` (`self.GetMovementComponent`)))
            (:`>`
              ;;[1 1 1] Correct Rotation for left and right sprite movement
              (`self.K2_SetActorRotation` (`KismetMathLibrary.MakeRotator` 0.0) :!label _label))
            (:`==`
              (if (`self.bisMovingRight`)
                (goto _label)
                (else
                  (`self.K2_SetActorRotation` (`KismetMathLibrary.MakeRotator` 0.0 0.0 180.0) :!label _label_2))))
            (:`<`
              (goto _label_2))))))))

(event `InputAxis MoveUp`
  (params (`Axis value` :type "Float (double-precision)"))
  ;[1 1 1] Handle movement
  (if (> `Axis value` 0.0)
    (set `self.bIsMovingUp` true)
    (elif (< `Axis value` 0.0)
      (set `self.bIsMovingUp` false)))
  (`self.AddMovementInput` (0.0 0.0 0.0) `Axis value`))

(fn `DestinationReached?`
  (set `self.DestinationReached` (== (`self.Destination`) (`SceneComponent.K2_GetComponentLocation` (`self.CapsuleComponent`)) :`ErrorTolerance` 250.0)))

(fn `DisplayForces`
  (`TextRenderComponent.K2_SetText` (`self.ForceStrengthTR`) (`KismetTextLibrary.Conv_DoubleToText` (`self.ImpulseStrength`) "HalfToEven"))
  (`TextRenderComponent.K2_SetText` (`self.ImpulseForceTR`) (`KismetTextLibrary.Conv_DoubleToText` (`self.ForceStrength`) "HalfToEven")))

(fn `SetDestination`
  (set `self.DestinationReached` false)
  (set `self.Destination` (`KismetMathLibrary.MakeVector` (`KismetMathLibrary.RandomFloatInRange` -3000.0 3000.0) 0.0 (`KismetMathLibrary.RandomFloatInRange` 250.0 3000.0))))

(fn `SetForces`
  (bind _radialforce (`self.RadialForce`))
  (set `RadialForceComponent.ForceStrength` (`self.ForceStrength`) _radialforce)
  (set `RadialForceComponent.ImpulseStrength` (`self.ImpulseStrength`) _radialforce)
  (set `RadialForceComponent.Radius` (`self.Radius`) _radialforce))

(fn `ShowDestinationMarker`
  (`|SpawnActorFromClass` null (`KismetMathLibrary.MakeTransform` (`self.Destination`)) "AlwaysSpawn" "OverrideRootScale" null null))

(fn `UserConstructionScript`)