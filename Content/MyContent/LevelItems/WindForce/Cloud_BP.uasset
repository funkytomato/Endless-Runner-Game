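; Cloud_BP is a wind-force level item that configures a radial force from its strength, impulse and radius variables.
; On BeginPlay it copies those variables into the RadialForce component and shows the two strengths on text render components.
; The label names are crossed: ForceStrengthTR1 shows the impulse strength and ImpulseForceTR shows the force strength.
; The construction script is empty, so values apply only at play time.
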(event `self.ReceiveBeginPlay`
  (bind _radialforce (`self.RadialForce`))
  ;[1 1 1] OnBegin - Populate Physics Force values
  (`TextRenderComponent.K2_SetText` (`self.ForceStrengthTR1`) (`KismetTextLibrary.Conv_DoubleToText` (`self.ImpulseStrength`) "HalfToEven"))
  (`TextRenderComponent.K2_SetText` (`self.ImpulseForceTR`) (`KismetTextLibrary.Conv_DoubleToText` (`self.ForceStrength`) "HalfToEven"))
  (set `RadialForceComponent.ForceStrength` (`self.ForceStrength`) _radialforce)
  (set `RadialForceComponent.ImpulseStrength` (`self.ImpulseStrength`) _radialforce)
  (set `RadialForceComponent.Radius` (`self.Radius`) _radialforce))

(fn `UserConstructionScript`)