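; CoinPickup_BP is a coin pickup for the 2D side-scroller that adds random points to a saved score.
; When the 2DSideScrollerCharacter overlaps its Collision component, it checks for the MySaveGame slot.
; If the slot exists, it loads it, increases Score, saves immediately and destroys the coin.
; Otherwise it calls save with no object connected, awarding nothing and leaving the coin in place.
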(event `self.Collision.OnComponentBeginOverlap`
  (params (OverlappedComponent :type "PrimitiveComponent Object Reference") (OtherActor :type "Actor Object Reference") (OtherComp :type "PrimitiveComponent Object Reference") (OtherBodyIndex :type Integer) (bFromSweep :type Boolean) (SweepResult :type "HitResult Structure (by ref)"))
  (cast `/Game/MyContent/Characters/NinjaCharacter/2DSideScrollerCharacter` OtherActor)
  (`GameplayStatics.CreateSaveGameObject` "/Game/MyContent/SaveGame/2DCharacter/MySaveGame.MySaveGame_C")
  (set `self.MySaveGame` null)
  (bind _returnvalue (`GameplayStatics.DoesSaveGameExist` "MySaveGame"))
  (if _returnvalue
    (bind _returnvalue_2 (`GameplayStatics.LoadGameFromSlot` "MySaveGame"))
    (bind _asmy_save_game (cast `/Game/MyContent/SaveGame/2DCharacter/MySaveGame` _returnvalue_2))
    (bind _output_get (set `self.MySaveGameInstance` _asmy_save_game))
    (set `/Game/MyContent/SaveGame/2DCharacter/MySaveGame.Score` (+ (`/Game/MyContent/SaveGame/2DCharacter/MySaveGame.Score` _output_get) (`KismetMathLibrary.RandomIntegerInRange` 10 100)) _output_get)
    (`GameplayStatics.SaveGameToSlot` _output_get "MySaveGame")
    (`self.K2_DestroyActor`)
    (else
      (`GameplayStatics.SaveGameToSlot` null "MySaveGame"))))

(fn `UserConstructionScript`)