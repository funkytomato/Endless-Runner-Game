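; Kunai actor that damages Knight, BlackKnight and BronzeKnight enemies on contact.
; Its Sphere overlap runs a separate cast branch per knight type, subtracting a hardcoded amount directly from Health when the overlapped component is that knight's capsule.
; A capsule hit destroys the kunai immediately, while other components on a knight destroy it after a short delay.
; Overlaps with other actors do nothing.
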(event `self.Sphere.OnComponentBeginOverlap`
  (params (OverlappedComponent :type "PrimitiveComponent Object Reference") (OtherActor :type "Actor Object Reference") (OtherComp :type "PrimitiveComponent Object Reference") (OtherBodyIndex :type Integer) (bFromSweep :type Boolean) (SweepResult :type "HitResult Structure (by ref)"))
  (`|ExecutionSequence`
    (:`then_0`
      ;[1 1 1] Damage Knight
      (bind _asknight_bp (cast `/Game/MyContent/Enemies/Knight/Knight_BP` OtherActor))
      (if (== (`/Game/MyContent/Enemies/Knight/Knight_BP.CapsuleCollision` _asknight_bp) OtherComp)
        (set `/Game/MyContent/Enemies/Knight/Knight_BP.Health` (- (`/Game/MyContent/Enemies/Knight/Knight_BP.Health` _asknight_bp) 26.0) _asknight_bp)
        (else
          (`KismetSystemLibrary.Delay` 2.0)))
      (`self.K2_DestroyActor`))
    (:`then_1`
      ;[1 1 1] Damage BlackKnight
      (bind _asblack_knight_bp (cast `/Game/MyContent/Enemies/BlackKnight/BlackKnight_BP` OtherActor))
      (if (== (`/Game/MyContent/Enemies/BlackKnight/BlackKnight_BP.CapsuleCollision` _asblack_knight_bp) OtherComp)
        (set `/Game/MyContent/Enemies/BlackKnight/BlackKnight_BP.Health` (- (`/Game/MyContent/Enemies/BlackKnight/BlackKnight_BP.Health` _asblack_knight_bp) 35.0) _asblack_knight_bp)
        (else
          (`KismetSystemLibrary.Delay` 2.0)))
      (`self.K2_DestroyActor`))
    (:`then_2`
      ;[1 1 1] Damage BronzeKnight
      (bind _asbronze_knight_bp (cast `/Game/MyContent/Enemies/BronzeKnight/BronzeKnight_BP` OtherActor))
      (if (== (`Character.CapsuleComponent` _asbronze_knight_bp) OtherComp)
        (set `/Game/MyContent/Enemies/BronzeKnight/BronzeKnight_BP.Health` (- (`/Game/MyContent/Enemies/BronzeKnight/BronzeKnight_BP.Health` _asbronze_knight_bp) 35.0) _asbronze_knight_bp)
        (else
          (`KismetSystemLibrary.Delay` 2.0)))
      (`self.K2_DestroyActor`))))

(fn `UserConstructionScript`)